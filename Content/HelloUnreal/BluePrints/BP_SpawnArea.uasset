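; BP_SpawnArea is an area actor that scatters rocks and red balls inside its Box volume.
; Its SpawnRRock event, which nothing in this graph calls, runs two loops in sequence to spawn a batch of BP_Rock, then BP_RedBall.
; Each spawn is half scale at a random point within the box's scaled extent.
; Disconnected leftover nodes for a counter-based spawn limit and a loop note never run.
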(event `SpawnRRock`
  (bind _box (`self.Box`))
  (bind _box_2 (`self.Box`))
  (`|ExecutionSequence`
    (:`then_0`
      (for _ (range 1 6)
        (`|SpawnActorFromClass` "/Game/HelloUnreal/BluePrints/BP_Rock.BP_Rock_C" (`KismetMathLibrary.MakeTransform` (`KismetMathLibrary.RandomPointInBoundingBox` (`SceneComponent.K2_GetComponentLocation` _box_2) (`BoxComponent.GetScaledBoxExtent` _box_2)) (struct) (0.5 0.5 0.5)) "Undefined" "MultiplyWithRoot" null null)))
    (:`then_1`
      (for _ (range 1 11)
        (`|SpawnActorFromClass` "/Game/HelloUnreal/BluePrints/BP_RedBall.BP_RedBall_C" (`KismetMathLibrary.MakeTransform` (`KismetMathLibrary.RandomPointInBoundingBox` (`SceneComponent.K2_GetComponentLocation` _box) (`BoxComponent.GetScaledBoxExtent` _box)) (struct) (0.5 0.5 0.5)) "Undefined" "MultiplyWithRoot" null null)))))

(fn `UserConstructionScript`)