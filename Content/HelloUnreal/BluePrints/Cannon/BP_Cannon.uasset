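; BP_Cannon is a cannon actor that toggles automatic firing of cannonballs when its F-press handler is called.
; EventPressF calls CannonFire, which flips a toggle to either fire at once and start a looping one-second timer, or clear that timer.
; Each shot spawns a BP_CannonBall at the Arrow component's world location and rotation.
; Start and EventReleaseF do nothing.
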(event `CannonFire`
  (bind _output_get (set `self.Toggle` (not (`self.Toggle`))))
  (if _output_get
    (`self.ShootCannon`)
    (`KismetSystemLibrary.K2_SetTimer` null "ShootCannon" 1.0 true)
    (else
      (`KismetSystemLibrary.K2_ClearTimer` null "ShootCannon"))))

(fn `EventPressF`
  (params (Character :type "Character Object Reference"))
  (returns (IsFail :type Boolean))
  (`self.CannonFire`)
  (return false))

(fn `EventReleaseF`
  (returns (IsFail :type Boolean))
  (return false))

(fn `ShootCannon`
  (bind (_returnvalue_location _returnvalue_rotation) (`KismetMathLibrary.BreakTransform` (`SceneComponent.K2_GetComponentToWorld` (`self.Arrow`))))
  (`|SpawnActorFromClass` "/Game/HelloUnreal/BluePrints/Cannon/BP_CannonBall.BP_CannonBall_C" (`KismetMathLibrary.MakeTransform` _returnvalue_location _returnvalue_rotation) "Undefined" "MultiplyWithRoot" null null))

(fn `Start`
  (params (IsPlay :type Boolean :default false))
  (returns (bIsResult :type Boolean)))

(fn `UserConstructionScript`)