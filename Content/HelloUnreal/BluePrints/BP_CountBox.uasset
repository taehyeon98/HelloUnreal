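; BP_CountBox is an interactive counter box that advances a single-digit count when a character presses F on it.
; EventPressF triggers CounterStart, which increments Count with wrap to zero at ten and shows it on a TextRender.
; It then broadcasts the new value through the ChangeCount event dispatcher for listeners.
; EventReleaseF and Start have no behavior.
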(event `CounterStart`
  (`self.Counting`)
  (`self.ShowCount`)
  (`self.EventDispatcher_ChangeCount` (`self.Count`)))

(fn `Counting`
  (set `self.Count` (+ (`self.Count`) 1))
  (if (>= (`self.Count`) 10)
    (set `self.Count` 0)))

(fn `EventPressF`
  (params (Character :type "Character Object Reference"))
  (returns (IsFail :type Boolean))
  (`self.CounterStart`)
  (return false))

(fn `EventReleaseF`
  (returns (IsFail :type Boolean))
  (return false))

(fn `ShowCount`
  (`TextRenderComponent.K2_SetText` (`self.TextRender`) (`KismetTextLibrary.Conv_IntToText` (`self.Count`))))

(fn `Start`
  (params (IsPlay :type Boolean :default false))
  (returns (bIsResult :type Boolean)))

(fn `UserConstructionScript`)