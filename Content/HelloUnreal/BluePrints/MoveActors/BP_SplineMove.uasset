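; BP_SplineMove is an actor that moves its Cube along a Spline in a repeating loop, started and stopped by a referenced Switch.
; A Timeline value scaled by spline length sets the Cube's world location and rotation, replaying from the start when finished.
; On BeginPlay it binds to the Switch's PlayStop dispatcher, or prints a warning if none is valid.
; Boolean handler functions route to the Start and Stop events.
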(event `Start`
  (bind (_direction _value) (`Timeline|Timeline` :!label _label)
    (:`Update`
      (bind (_returnvalue_location _returnvalue_rotation) (`KismetMathLibrary.BreakTransform` (`SplineComponent.GetTransformAtDistanceAlongSpline` (`self.Spline`) (* (`SplineComponent.GetSplineLength` (`self.Spline`)) _value) "World" false)))
      (`SceneComponent.K2_SetWorldLocationAndRotation` (`self.Cube`) _returnvalue_location _returnvalue_rotation false false))
    (:`Finished`
      (goto _label :!via `PlayFromStart`))))

(event `Stop`
  (goto _label :!via `Stop`))

(event `self.ReceiveBeginPlay`
  (bind _switch (`self.Switch`)
    (:`then`
      (add `/Game/HelloUnreal/BluePrints/BP_Switch.EventDispatcher_PlayStop` _switch (`|CreateDelegate` :!event `BP_SplineMove_AutoGenFunc`)))
    (:`else`
      (`KismetSystemLibrary.PrintString` "Forget SplineMove" true true (struct :`R` 1.0 :`A` 1.0)))))

(fn `BP_SplineMove_AutoGenFunc`
  (params (Toggle :type Boolean))
  (if Toggle
    (`self.Start`)
    (else
      (`self.Stop`))))

(fn `EventPlay`
  (params (IsPlay :type Boolean :default false))
  (returns (bIsResult :type Boolean))
  (if IsPlay
    (`self.Start`)
    (else
      (`self.Stop`)))
  (return false))

(fn `UserConstructionScript`)