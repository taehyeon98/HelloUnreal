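; BP_LeftRightTL is a switch-controlled moving actor that slides its Cube back and forth with a Timeline.
; The Timeline value scales the Scene component's relative location to position the Cube, and each finish flips IsMoveRight to reverse direction.
; BeginPlay binds to the Switch's play/stop dispatcher, or prints a warning when no Switch is valid.
; EventPlayStop and EventPlay each start or stop the motion from a boolean.
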(event `Start`
  (if (`self.IsMoveRight`) :!label _label
    (bind (_direction _value) (`Timeline|Timeline` :!label _label_2)
      (:`Update`
        (`SceneComponent.K2_SetRelativeLocation` (`self.Cube`) (* _value (`SceneComponent.RelativeLocation` (`self.Scene`))) false false))
      (:`Finished`
        (set `self.IsMoveRight` (not (`self.IsMoveRight`)))
        (goto _label)))
    (else
      (goto _label_2 :!via `Reverse`))))

(event `Stop`
  (goto _label_2 :!via `Stop`))

(event `self.ReceiveBeginPlay`
  (bind _switch (`self.Switch`)
    (:`then`
      (add `/Game/HelloUnreal/BluePrints/BP_Switch.EventDispatcher_PlayStop` _switch (`|CreateDelegate` :!event `EventPlayStop`)))
    (:`else`
      (`KismetSystemLibrary.PrintString` "BP_LeftRightTL에 스위치 지정이 안되있음." true true (struct :`R` 1.0 :`A` 1.0)))))

(fn `EventPlay`
  (params (IsPlay :type Boolean :default false))
  (returns (bIsResult :type Boolean))
  (locals (NewLocalVar :type Boolean :default true))
  (if IsPlay
    (`self.Start`)
    (else
      (`self.Stop`)))
  (return false))

(fn `EventPlayStop`
  (params (Toggle :type Boolean))
  (if Toggle
    (`self.Start`)
    (else
      (`self.Stop`))))

(fn `UserConstructionScript`)