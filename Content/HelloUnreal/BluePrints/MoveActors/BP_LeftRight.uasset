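; BP_LeftRight is a moving actor that shuttles its Aaa component back and forth along relative X between 0 and 500.
; While IsPlay is set, Tick calls MoveRight or MoveLeft for fixed per-frame, frame-rate-dependent steps, flipping IsMoveRight at each limit.
; BeginPlay binds to the Swtich reference's PlayStop dispatcher for play/stop control, or prints a red warning if that reference is invalid.
; MoveRL duplicates the Tick logic but is not called here.
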(event `self.ReceiveTick`
  (params (DeltaSeconds :type "Float (single-precision)"))
  (if (`self.IsPlay`)
    (if (`self.IsMoveRight`)
      ; 오른쪽으로 움직인다.
      (`self.MoveRight`)
      (if (>= (`self.LocationX`) 500.0)
        (set `self.IsMoveRight` false))
      (else
        ; 왼쪽으로 움직인다.
        (`self.MoveLeft`)
        (if (<= (`self.LocationX`) 0.0)
          (set `self.IsMoveRight` true))))))

(event `self.ReceiveBeginPlay`
  (bind _swtich (`self.Swtich`)
    (:`then`
      (add `/Game/HelloUnreal/BluePrints/BP_Switch.EventDispatcher_PlayStop` _swtich (`|CreateDelegate` :!event `BP_LeftRight_AutoGenFunc`)))
    (:`else`
      (`KismetSystemLibrary.PrintString` "Forget LeftRight" true true (struct :`R` 1.0 :`A` 1.0)))))

(fn `BP_LeftRight_AutoGenFunc`
  (params (Toggle :type Boolean))
  (set `self.IsPlay` Toggle))

(fn `EventPlay`
  (params (IsPlay :type Boolean :default false))
  (returns (bIsResult :type Boolean))
  (bind _output_get (set `self.IsPlay` IsPlay))
  (return _output_get))

(fn `MoveLeft`
  (bind _output_get (set `self.LocationX` (+ (`self.LocationX`) -1.0)))
  (`SceneComponent.K2_SetRelativeLocation` (`self.aaa`) (`KismetMathLibrary.MakeVector` _output_get) false false))

(fn `MoveRight`
  (bind _output_get (set `self.LocationX` (+ (`self.LocationX`) 1.0)))
  (`SceneComponent.K2_SetRelativeLocation` (`self.aaa`) (`KismetMathLibrary.MakeVector` _output_get) false false))

(fn `MoveRL`
  (if (`self.IsMoveRight`)
    (bind _output_get (set `self.LocationX` (+ (`self.LocationX`) 1.0)))
    (`SceneComponent.K2_SetRelativeLocation` (`self.aaa`) (`KismetMathLibrary.MakeVector` _output_get) false false)
    (if (>= (`self.LocationX`) 500.0)
      (set `self.IsMoveRight` false))
    (else
      (bind _output_get_2 (set `self.LocationX` (+ (`self.LocationX`) -1.0)))
      (`SceneComponent.K2_SetRelativeLocation` (`self.aaa`) (`KismetMathLibrary.MakeVector` _output_get_2) false false)
      (if (<= (`self.LocationX`) 0.0)
        (set `self.IsMoveRight` true)))))

(fn `UserConstructionScript`)