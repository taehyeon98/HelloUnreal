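; BP_Dummy is a damageable target dummy actor that shows its health on a widget component and destroys itself at zero HP.
; AnyDamage subtracts damage from CurHp and pushes current and max HP to the HPWidget, which BeginPlay also initializes.
; Every tick, LookPlayer rotates the widget toward the player camera using only X and Y positions as look-at inputs.
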(event `self.ReceiveAnyDamage`
  (params (Damage :type "Float (single-precision)") (DamageType :type "DamageType Object Reference") (InstigatedBy :type "Controller Object Reference") (DamageCauser :type "Actor Object Reference"))
  (set `self.CurHp` (- (`self.CurHp`) Damage))
  (bind _ashpwidget (cast `/Game/HelloUnreal/NameTag/HPWidget` (`WidgetComponent.GetUserWidgetObject` (`self.Widget`))))
  (`/Game/HelloUnreal/NameTag/HPWidget.SetHp` _ashpwidget (`self.CurHp`) (`self.MaxHp`))
  (if (<= (`self.CurHp`) 0.0)
    (`self.K2_DestroyActor`)))

(event `self.ReceiveTick`
  (params (DeltaSeconds :type "Float (single-precision)"))
  (`self.LookPlayer`))

(event `self.ReceiveBeginPlay`
  (bind _ashpwidget (cast `/Game/HelloUnreal/NameTag/HPWidget` (`WidgetComponent.GetUserWidgetObject` (`self.Widget`))))
  (`/Game/HelloUnreal/NameTag/HPWidget.SetHp` _ashpwidget (`self.CurHp`) (`self.MaxHp`)))

(fn `LookPlayer`
  (bind (_returnvalue_x _returnvalue_y) (`KismetMathLibrary.BreakVector` (`SceneComponent.K2_GetComponentLocation` (`self.Widget`))))
  (bind (_returnvalue_x_2 _returnvalue_y_2) (`KismetMathLibrary.BreakVector` (`PlayerCameraManager.GetCameraLocation` (`GameplayStatics.GetPlayerCameraManager` 0))))
  (`SceneComponent.K2_SetWorldRotation` (`self.Widget`) (`KismetMathLibrary.FindLookAtRotation` (`KismetMathLibrary.MakeVector` _returnvalue_x _returnvalue_y) (`KismetMathLibrary.MakeVector` _returnvalue_x_2 _returnvalue_y_2)) false false))

(fn `UserConstructionScript`)