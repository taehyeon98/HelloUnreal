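; BP_LeftRight is a practice actor that slides its Aaa component back and forth along the X axis.
; Each Tick steps LocationX by a fixed, frame-rate-dependent amount and flips IsMoveRight at the 0 and 500 limits.
; The Construction Script gives Aaa a dynamic instance of M_Mask_Inst and sets its Color parameter.
; BeginPlay only prints a string, and a set of unconnected math and comparison nodes remains in the EventGraph.
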(event `self.ReceiveBeginPlay`
  ; 이 액터가 플레이 될때
  ; 화면에 String 출력
  (`KismetSystemLibrary.PrintString` "Hello"))

(event `self.ReceiveTick`
  (params (DeltaSeconds :type "Float (single-precision)"))
  (if (`self.IsMoveRight`)
    ; 오른쪽으로 움직인다.
    (bind _output_get (set `self.LocationX` (+ (`self.LocationX`) 1.0)))
    (`SceneComponent.K2_SetRelativeLocation` (`self.aaa`) (`KismetMathLibrary.MakeVector` _output_get) false false)
    (if (>= (`self.LocationX`) 500.0)
      (set `self.IsMoveRight` false))
    (else
      ; 왼쪽으로 움직인다.
      (bind _output_get_2 (set `self.LocationX` (+ (`self.LocationX`) -1.0)))
      (`SceneComponent.K2_SetRelativeLocation` (`self.aaa`) (`KismetMathLibrary.MakeVector` _output_get_2) false false)
      (if (<= (`self.LocationX`) 0.0)
        (set `self.IsMoveRight` true)))))

(fn `UserConstructionScript`
  (bind _returnvalue (`PrimitiveComponent.CreateDynamicMaterialInstance` (`self.aaa`) 0 "/Game/HelloUnreal/StartUnreal/M_Mask_Inst.M_Mask_Inst" "None"))
  (`MaterialInstanceDynamic.SetVectorParameterValue` _returnvalue "Color" (`self.Value`)))