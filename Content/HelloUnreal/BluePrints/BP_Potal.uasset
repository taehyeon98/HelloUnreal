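; BP_Potal is a password-locked portal whose Sphere stays hidden until the linked count boxes show the correct combination.
; On BeginPlay it hides the Sphere and binds to each box's ChangeCount dispatcher.
; EventChangingCount sets Sphere visibility from CheckArrPassword, which compares each box's Count to ArrPassword by index.
; An alternative CheckPassword, which extracts digits from an integer Password using modulo and division, is not used by that handler.
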(event `self.ReceiveBeginPlay`
  (`SceneComponent.SetVisibility` (`self.Sphere`) false false)
  ; 각각의 액터값 확인
  (for _array_element (`self.CountBoxes`)
    (add `/Game/HelloUnreal/BluePrints/BP_CountBox.EventDispatcher_ChangeCount` _array_element (`|CreateDelegate` :!event `EventChangingCount`))))

(fn `CheckArrPassword`
  (returns (IsAll9 :type Boolean))
  (for (_array_element _array_index) (`self.CountBoxes`)
    (if (not (== (`/Game/HelloUnreal/BluePrints/BP_CountBox.Count` _array_element) (`|GetArrayItem` (`self.ArrPassword`) _array_index)))
      (return false)))
  (return true))

(fn `CheckPassword`
  (returns (IsAll9 :type Boolean))
  ; 카운터박스개수만큼 돈다
  (for (_array_element _array_index) (`self.CountBoxes`)
    ; 하나라도 값이 9가 아니면
    (if (not (== (`/Game/HelloUnreal/BluePrints/BP_CountBox.Count` _array_element) (`self.IndexToPassword` _array_index)))
      (return false)))
  ; 3개다 9
  (return true))

(fn `EventChangingCount`
  (params (Count :type Integer))
  (`SceneComponent.SetVisibility` (`self.Sphere`) (`self.CheckArrPassword`) false))

(fn `GetNumberToCount0`
  (params (Number :type Integer))
  (returns (ResultCount0 :type Integer))
  (locals (Count0 :type Integer :default 1))
  (for _ (range 1 (+ Number 1))
    (set `local.Count0` (* (`local.Count0`) 10)))
  (return (`local.Count0`)))

(fn `IndexToPassword`
  (params (Index :type Integer))
  (returns (Password :type Integer))
  (bind _returnvalue (- (`KismetArrayLibrary.Array_Length` (`self.CountBoxes`)) Index))
  (return (/ (mod (`self.Password`) (`self.GetNumberToCount0` _returnvalue)) (`self.GetNumberToCount0` (- _returnvalue 1)))))

(fn `UserConstructionScript`)