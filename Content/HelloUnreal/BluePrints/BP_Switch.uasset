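; BP_Switch is an interactable switch that toggles a play/stop state when F is pressed.
; EventPressF calls Play, which flips Toggle and passes the new value to CallEventDispatcherPlayStop to notify listeners.
; Start, EventPlay and EventReleaseF are stubs that return false, and the event graph also holds disconnected example nodes for array operations and overlap logging, some with Korean notes.
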(event `Play`
  (bind _output_get (set `self.Toggle` (not (`self.Toggle`))))
  (`self.EventDispatcher_PlayStop` _output_get))

(fn `EventPlay`
  (params (IsPlay :type Boolean))
  (returns (bIsResult :type Boolean))
  (return false))

(fn `EventPressF`
  (params (Character :type "Character Object Reference"))
  (returns (IsFail :type Boolean))
  (`self.Play`)
  (return false))

(fn `EventReleaseF`
  (returns (IsFail :type Boolean))
  (return false))

(fn `Start`
  (params (IsPlay :type Boolean :default false))
  (returns (bIsResult :type Boolean))
  (return false))

(fn `UserConstructionScript`)