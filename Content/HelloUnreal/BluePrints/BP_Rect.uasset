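; BP_Rect is an actor that moves its Aaa component back and forth along an L-shaped path in the relative XZ plane.
; Tick switches on MoveType, stepping LocationX or LocationZ by a fixed, frame-rate-dependent amount and changing state at each limit.
; The cycle runs Right, Up, Down, Left, so it retraces two edges instead of tracing a full rectangle.
; BeginPlay only prints a string.
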(event `self.ReceiveBeginPlay`
  ; 이 액터가 플레이 될때
  ; 화면에 String 출력
  (`KismetSystemLibrary.PrintString` "Hello"))

(event `self.ReceiveTick`
  (params (DeltaSeconds :type "Float (single-precision)"))
  (switch `/Game/HelloUnreal/BluePrints/EN_MoveType` (`self.MoveType`)
    (:`NewEnumerator9`
      ; 오른쪽으로 움직인다.
      (bind _output_get (set `self.LocationX` (+ (`self.LocationX`) 1.0)))
      (`SceneComponent.K2_SetRelativeLocation` (`self.aaa`) (`KismetMathLibrary.MakeVector` _output_get 0.0 (`self.LocationZ`)) false false)
      (if (>= (`self.LocationX`) 500.0)
        (set `self.MoveType` "NewEnumerator10")))
    (:`NewEnumerator10`
      ; 위로 움직인다.
      (bind _output_get_2 (set `self.LocationZ` (+ (`self.LocationZ`) 1.0)))
      (`SceneComponent.K2_SetRelativeLocation` (`self.aaa`) (`KismetMathLibrary.MakeVector` (`self.LocationX`) 0.0 _output_get_2) false false)
      (if (>= (`self.LocationZ`) 500.0)
        (set `self.MoveType` "NewEnumerator12")))
    (:`NewEnumerator11`
      ; 왼쪽으로 움직인다.
      (bind _output_get_3 (set `self.LocationX` (+ (`self.LocationX`) -1.0)))
      (`SceneComponent.K2_SetRelativeLocation` (`self.aaa`) (`KismetMathLibrary.MakeVector` _output_get_3 0.0 (`self.LocationZ`)) false false)
      (if (<= (`self.LocationX`) 0.0)
        (set `self.MoveType` "NewEnumerator9")))
    (:`NewEnumerator12`
      ; 아래로 움직인다.
      (bind _output_get_4 (set `self.LocationZ` (+ (`self.LocationZ`) -1.0)))
      (`SceneComponent.K2_SetRelativeLocation` (`self.aaa`) (`KismetMathLibrary.MakeVector` (`self.LocationX`) 0.0 _output_get_4) false false)
      (if (<= (`self.LocationZ`) 0.0)
        (set `self.MoveType` "NewEnumerator11")))))

(fn `UserConstructionScript`)