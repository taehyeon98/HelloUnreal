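; BP_LeftRightTL is an actor that moves its Cube back and forth in a continuous loop from BeginPlay.
; A Timeline scales the Scene component's relative location by its value to set the Cube's relative location, so Scene acts as a movable travel marker.
; Each time the Timeline finishes, it flips IsMoveRight and loops back to either play forward or reverse, creating a ping-pong without Tick.
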(event `self.ReceiveBeginPlay`
  (if (`self.IsMoveRight`) :!label _label
    (bind (_direction _value) (`Timeline|Timeline` :!label _label_2)
      (:`Update`
        (`SceneComponent.K2_SetRelativeLocation` (`self.Cube`) (* _value (`SceneComponent.RelativeLocation` (`self.Scene`))) false false))
      (:`Finished`
        (set `self.IsMoveRight` (not (`self.IsMoveRight`)))
        (goto _label)))
    (else
      (goto _label_2 :!via `Reverse`))))

(fn `UserConstructionScript`)